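; Test-style actor that imitates a prefab of destructible rock components, spawning and shattering them as soon as play begins.
; A loop adds about 160 scaled-up DestructibleComponents at random points within the Box bounds, all using one cover-rock destructible mesh.
; Each iteration sets a large-chunk threshold, adds a CHRoleWriter component, then applies radius damage with impulse at the new component's location to break it immediately.
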(event `self.ReceiveBeginPlay`
  (`self.SpawnAndBlowUp`))

(event `SpawnAndBlowUp`
  (for _ (range 161)
    (bind _returnvalue (`AddComponent|NODE_AddDestructibleComponent-0` :`RelativeTransform` (`KismetMathLibrary.MakeTransform` (`KismetMathLibrary.RandomPointInBoundingBox` (0.0 0.0 0.0) (`.BoxExtent` (`KismetSystemLibrary.GetComponentBounds` (`self.Box`)))) (struct) (5.0 5.0 5.0))))
    (`DestructibleComponent.SetDestructibleMesh` _returnvalue "/Game/RedwoodCollection/Meshes/Cover/SM_RW_Cover_Rock05_DM.SM_RW_Cover_Rock05_DM")
    (set `DestructibleComponent.LargeChunkThreshold` 2500.0 _returnvalue)
    (`AddComponent|NODE_AddCHRoleWriter-0`)
    (`DestructibleComponent.ApplyRadiusDamage` _returnvalue 100.0 (`SceneComponent.K2_GetComponentLocation` _returnvalue) 100.0 10000.0 false)))

(fn `UserConstructionScript`)