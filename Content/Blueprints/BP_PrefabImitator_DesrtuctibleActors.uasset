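; Client-only effect actor that imitates a burst of shattering rock debris inside its box bounds.
; On BeginPlay a short looping timer spawns batches of destructible rock actors at random points in the box.
; Each gets a destructible mesh and a CH role writer, then immediate radius damage breaks it apart.
; After a few batches the timer stops, and following a delay the spawned actors and the imitator destroy themselves.
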(event `self.ReceiveBeginPlay`
  (`/Engine/EditorBlueprintResources/ActorMacros.Switch Has Authority`
    (:`Remote`
      (bind _returnvalue (`KismetSystemLibrary.K2_SetTimerDelegate` (delegate `SpawnTimerFunction`) 0.1 true))
      (set `self.TimerHandle` _returnvalue))))

(event `SpawnTimerFunction`
  (bind (_origin _boxextent) (`KismetSystemLibrary.GetComponentBounds` (`self.Box`)))
  (for _ (range 4)
    (bind _returnvalue (`|SpawnActorFromClass` "/Script/ApexDestruction.DestructibleActor" (`KismetMathLibrary.MakeTransform` (`KismetMathLibrary.RandomPointInBoundingBox` _origin _boxextent) (struct) (2.0 2.0 2.0)) "AlwaysSpawn" "OverrideRootScale" self null))
    (`KismetArrayLibrary.Array_Add` (`self.ActorsForRemove`) _returnvalue)
    (bind _destructiblecomponent (`DestructibleActor.DestructibleComponent` _returnvalue))
    (`DestructibleComponent.SetDestructibleMesh` _destructiblecomponent "/Game/RedwoodCollection/Meshes/Cover/SM_RW_Cover_Rock05_DM.SM_RW_Cover_Rock05_DM")
    (set `DestructibleComponent.LargeChunkThreshold` 2500.0 _destructiblecomponent)
    (`AddComponent|NODE_AddCHRoleWriter-0` :`self` _returnvalue)
    (`DestructibleComponent.ApplyRadiusDamage` _destructiblecomponent 100.0 (`self.K2_GetActorLocation` _returnvalue) 100.0 10000.0 false))
  (bind _result (`/Engine/EditorBlueprintResources/StandardMacros.IncrementInt` (`self.TimerCounter`))
    (:`  `
      (if (>= _result 4)
        (`KismetSystemLibrary.K2_ClearAndInvalidateTimerHandle` (`self.TimerHandle`))
        (`KismetSystemLibrary.Delay` 4.0)
        (for _array_element (`self.ActorsForRemove`)
          (if (`KismetSystemLibrary.IsValid` _array_element)
            (`self.K2_DestroyActor` _array_element)))
        (`self.K2_DestroyActor`)))))

(fn `UserConstructionScript`)